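; Base AI controller that runs the BaseBT behavior tree on BeginPlay and feeds its Blackboard from AI Perception updates.
; Sight of an actor tagged Player sets TargetActor, and losing sight clears it.
; Hearing stimuli whose tag is in PerceptionTags write their location to TargetHearedLocation, which this controller never clears.
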(event `self.ReceiveBeginPlay`
  (`self.RunBehaviorTree` "/Game/NeonV/AI/BaseBT.BaseBT"))

(event `self.AIPerception.OnTargetPerceptionUpdated`
  (params (Actor :type "Actor Object Reference") (Stimulus :type "AIStimulus Structure"))
  (bind (_age _expirationage _strength _stimuluslocation _receiverlocation _tag _bsuccessfullysensed) (break `AIStimulus` Stimulus))
  (bind _blackboard (`self.Blackboard`))
  (bind _returnvalue (`AIPerceptionSystem.GetSenseClassForStimulus` Stimulus))
  (if (== _returnvalue "/Script/AIModule.AISense_Sight")
    (if (`self.ActorHasTag` Actor "Player")
      (if _bsuccessfullysensed
        (`BlackboardComponent.SetValueAsObject` _blackboard "TargetActor" Actor)
        (else
          (`BlackboardComponent.ClearValue` _blackboard "TargetActor"))))
    (elif (== _returnvalue "/Script/AIModule.AISense_Hearing")
      (if (`BlueprintMapLibrary.Map_Contains` (`self.PerceptionTags`) _tag)
        (`BlackboardComponent.SetValueAsVector` (`self.Blackboard`) "TargetHearedLocation" _stimuluslocation)))))

(fn `UserConstructionScript`)